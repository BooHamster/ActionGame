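; BP_Enemy4 is a red-tinted 2D flipbook zombie enemy that chases and bites the player.
; PawnSensing turns it toward the player and starts AIMoveTo, whose success triggers a delay-timed bite where HitCheck damages characters overlapping HitBox.
; Damage redirects its movement to a fixed point, then either stuns it or plays death and destroys it.
; Finished flipbooks return it to idle unless dead; frame-based hit timing is left unconnected.
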(event OnSeePawn(PawnSensing)
  (params (Pawn :type Pawn%20Object%20Reference))
  (bind _capsulecomponent (Variables|Collision|GetCapsuleComponent))
  ;[1 1 1] Player tracking and setting the attack animation
  (if (not (Variables|Default|GetIsDead))
    ;;[1 1 1] Player tracking and setting the attack animation
    (if (not (Variables|Default|GetStunned))
      (if (not (Variables|Default|GetIsAttacking))
        (Variables|Default|SetIsSeeingPlayer true)
        (CallFunction|FollowPlayer)
        ;[1 1 1] Face Player
        (if (>= (.x (Math|Vector|Normalize (- (Transformation|GetActorLocation) (Transformation|GetActorLocation (Variables|Default|GetCHR%20ref))))) 0.0)
          (Transformation|SetWorldRotation _capsulecomponent "180.000000,0.000000,0.000000" false false)
          (else
            (Transformation|SetWorldRotation _capsulecomponent "0, 0, 0" false false)))))))

(event OnFinishedPlaying(Sprite)
  ;[1 1 1] Reset the idle animation from attack or hurt animation
  (if (not (Variables|Default|GetIsDead))
    (Components|Timeline|SetLooping (Variables|Default|GetSprite) false)
    (Development|SetHiddeninGame (Variables|Default|GetHitBox) true false)
    (Sprite|SetFlipbook (Variables|Default|GetSprite) "/Game/Enemies/ZombieMan/Idle/FB_ZombieIdle.FB_ZombieIdle")
    (Components|Timeline|SetLooping (Variables|Default|GetSprite) true)
    (if (not (Audio|Components|Audio|IsPlaying (Variables|Default|GetSprite)))
      (Audio|Components|Audio|Play (Variables|Default|GetSprite)))))

(event Custom|ResetAttack
  ;[1 1 1] Player tracking and setting the attack animation
  (Utilities|FlowControl|DoOnce true) ; enters at Reset
)

(event Custom|FollowPlayer
  (bind _sprite (Variables|Default|GetSprite))
  ;[1 1 1] Player tracking and setting the attack animation
  (if (Variables|Default|GetIsSeeingPlayer)
    (Sprite|SetFlipbook (Variables|Default|GetSprite) "/Game/Enemies/ZombieMan/Walk/FB_ZombieWalk.FB_ZombieWalk")
    (AI|AIMoveTo self "0, 0, 0" (Game|GetPlayerCharacter 0) 15.0 false
      (:OnSuccess
        (if (not (Variables|Default|GetIsAttacking))
          (Variables|Default|SetIsAttacking true)
          (Sprite|SetFlipbook _sprite "/Game/Enemies/ZombieMan/Attack/FB_ZombieBite.FB_ZombieBite")
          ;;[1 1 1] Player tracking and setting the attack animation
          (Components|Timeline|SetLooping _sprite false)
          (Utilities|FlowControl|Delay 0.5)
          (if (not (Variables|Default|GetStunned))
            (if (not (Variables|Default|GetIsDead))
              (CallFunction|HitCheck)
              (Development|SetHiddeninGame (Variables|Default|GetHitBox) false false)
              (Utilities|FlowControl|Delay 0.1)
              (Development|SetHiddeninGame (Variables|Default|GetHitBox) true false)
              (Utilities|FlowControl|Delay 1.0)
              (Variables|Default|SetIsAttacking false)
              (CallFunction|ResetAttack))))))))

(event Collision|EventActorBeginOverlap
  (params (OtherActor :type Actor%20Object%20Reference))
  ;[1 1 1] Player tracking and setting the attack animation
)

(event EventBeginPlay
  (bind _aspaper_character (Utilities|Casting|CastToPaperCharacter (Game|GetPlayerCharacter 0)))
  (Variables|Default|SetCHR%20ref _aspaper_character)
  (Sprite|SetSpriteColor (Variables|Default|GetSprite) "(R=0.601191,G=0.000000,B=0.013427,A=1.000000)"))

(event EventTick
  (params (DeltaSeconds :type Float%20%28single-precision%29))
  ;[1 1 1] Choosing which frame to spawn hitbox and cause damage from basic attack
)

(event Game|Damage|EventAnyDamage
  (params (Damage :type Float%20%28single-precision%29) (DamageType :type Damage%20Type%20Object%20Reference) (InstigatedBy :type Controller%20Object%20Reference) (DamageCauser :type Actor%20Object%20Reference))
  (bind _sprite (Variables|Default|GetSprite))
  ;[1 1 1] Taking Damage
  (Development|PrintString (Utilities|String|ToString(Float) Damage))
  (Variables|Default|SetHealth (- (Variables|Default|GetHealth) Damage))
  (AI|AIMoveTo self "50.000000,50.000000,0.000000" 0 5.0 false
    (:then
      _)
    (:OnSuccess
      _))
  (if (<= (Variables|Default|GetHealth) 0.0)
    (Sprite|SetFlipbook _sprite "/Game/Enemies/ZombieMan/Dead/FB_ZombieDead.FB_ZombieDead")
    (Components|Timeline|SetLooping _sprite false)
    (Collision|SetCollisionEnabled (Variables|Collision|GetCapsuleComponent) "NoCollision")
    (Variables|Default|SetIsDead true)
    (Utilities|FlowControl|Delay 3.0)
    (Actor|DestroyActor)
    (else
      (Sprite|SetFlipbook _sprite "/Game/Enemies/ZombieMan/Hurt/FB_ZombieHurt.FB_ZombieHurt")
      (Components|Timeline|SetLooping _sprite false)
      (Variables|Default|SetStunned true)
      (Variables|Default|SetIsSeeingPlayer false)
      (Utilities|FlowControl|Delay (Variables|Default|GetStunDuration))
      (Variables|Default|SetStunned false)
      (Variables|Default|SetIsAttacking false))))

(fn ConstructionScript)

(fn HitCheck
  (for _array_element (Collision|GetOverlappingActors (Variables|Default|GetHitBox) "/Game/TestausHahmo/BP_Character.BP_Character_C" :!class /Script/Engine.PrimitiveComponent)
    (if (!= _array_element self)
      (Game|Damage|ApplyDamage _array_element (Variables|Default|GetDamageAmount) 0 0)
      (LocalVariables|SetHitSomething true)
      (Audio|PlaySound2D "/Engine/VREditor/Sounds/UI/Laser_Pull.Laser_Pull" 1.0 1.0 0.0 0 0)))
  (if (LocalVariables|GetHitSomething)
    (Effects|SpawnEmitteratLocation 0 (Transformation|GetSocketLocation (Variables|Default|GetSprite) "HitPos") "0, 0, 0" "0.100000,0.100000,0.100000")
    (Audio|PlaySound2D "/Engine/VREditor/Sounds/UI/Laser_Push.Laser_Push" 1.0 1.0 0.0 0 0)))